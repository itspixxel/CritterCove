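; Basic rifle weapon Blueprint that handles firing and reloading with first-person montages on the player's Mesh1P.
; Fire is blocked while reloading; otherwise it starts the fire montage and immediately calls FireHitScan.
; Reload sets IsReloading and plays the reload montage, clearing the flag on blend out or after a short delay if interrupted.
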(event EventBeginPlay
  (|CallParentFunction) ; This node is disabled and will not be called.\nDrag off pins to build functionality.
)

(event Collision|EventActorBeginOverlap
  (params (OtherActor :type Actor%20Object%20Reference)))

(event EventTick
  (params (DeltaSeconds :type Float%20%28single-precision%29)))

(event EventFire
  (if (not (Variables|Default|GetbIsReloading))
    (Animation|Montage|PlayMontage (Variables|/Game/Assets/Blueprints/GameBP/BP_CritterCoveCharacterOld.BP_CritterCoveCharacterOld_C|GetMesh1P (Variables|Default|GetPlayerRef)) "/Game/Assets/Animations/FP_Fire_Montage.FP_Fire_Montage"
      (:then
        (CallFunction|FireHitScan true)))))

(event EventReload
  (if (not (Variables|Default|GetbIsReloading))
    (Variables|Default|SetbIsReloading true)
    (Animation|Montage|PlayMontage (Variables|/Game/Assets/Blueprints/GameBP/BP_CritterCoveCharacterOld.BP_CritterCoveCharacterOld_C|GetMesh1P (Variables|Default|GetPlayerRef)) "/Game/Assets/Animations/FP_Reload_Montage.FP_Reload_Montage"
      (:OnBlendOut
        (Variables|Default|SetbIsReloading false))
      (:OnInterrupted
        (Utilities|FlowControl|Delay 1.0)
        (Variables|Default|SetbIsReloading false)))))

(fn ConstructionScript
  (|CallParentFunction))