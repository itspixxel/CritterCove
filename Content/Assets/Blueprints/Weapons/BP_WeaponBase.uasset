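; BP_WeaponBase is a base weapon Blueprint, attached as a child actor of BP_CritterCoveCharacter, with empty Equip, Stow, Fire and Reload events.
; The construction script applies the configured mesh and material, and BeginPlay caches the parent character.
; FireHitScan traces from the first-person camera within a random spread cone and stores that hit.
; It then traces from the muzzle toward that aim point, optionally debug-drawn, but leaves this result unused.
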(event Custom|Reload
  ;[0.15 0.15 0.15 0.5] Events
)

(event Custom|Equip
  ;[0.15 0.15 0.15 0.5] Events
)

(event Custom|Stow
  ;[0.15 0.15 0.15 0.5] Events
)

(event Custom|Fire
  ;[0.15 0.15 0.15 0.5] Events
)

(event EventBeginPlay
  ;[0.15 0.15 0.15 0.5] Get Player Reference
  (bind _asbp_critter_cove_character (Utilities|Casting|CastToBP_CritterCoveCharacter (Actor|GetParentActor)))
  (Variables|Default|SetPlayerRef _asbp_critter_cove_character))

(fn ConstructionScript
  (Components|SkeletalMesh|SetSkeletalMeshAsset (Variables|Default|GetWeaponMesh) (Variables|Default|GetMesh))
  (Rendering|Material|SetMaterial (Variables|Default|GetWeaponMesh) 0 (Variables|Default|GetMaterial)))

(fn FireHitScan
  (params (DrawDebug :type Boolean))
  (bind _playerref (Variables|Default|GetPlayerRef))
  (bind _firstpersoncamera (Variables|/Game/Assets/Blueprints/GameBP/BP_CritterCoveCharacter.BP_CritterCoveCharacter_C|GetFirstPersonCamera _playerref))
  (bind _returnvalue (Transformation|GetWorldLocation _firstpersoncamera))
  (bind _returnvalue_2 (Math|Vector|GetForwardVector _firstpersoncamera))
  (bind (_outhit _returnvalue_3) (Collision|LineTraceByChannel _returnvalue (+ _returnvalue (* (Math|Random|RandomUnitVectorinConeinDegrees _returnvalue_2 (Variables|Default|GetSpread)) (Variables|Default|GetRange))) "TraceTypeQuery1" false (Utilities|Array|MakeArray (Variables|Default|GetPlayerRef)) "None"))
  (LocalVariables|SetLoc_HitInfo _outhit)
  (Collision|LineTraceByChannel (Transformation|GetSocketLocation (Variables|Default|GetWeaponMesh) "Muzzle") (Math|Vector|SelectVector (+ (.Location (Collision|BreakHitResult _outhit)) (* _returnvalue_2 1e+01)) (.TraceEnd (Collision|BreakHitResult _outhit)) _returnvalue_3) "TraceTypeQuery1" false (Utilities|Array|MakeArray (Variables|Default|GetPlayerRef)) (select DrawDebug "ForDuration" "None")))